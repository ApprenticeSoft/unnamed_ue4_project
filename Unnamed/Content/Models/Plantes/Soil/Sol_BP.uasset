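; Soil plot actor Blueprint that shows a selection square when it is selected.
; On BeginPlay it takes the Soil_Widget_BP from its widget component and stores it.
; SetSelected and SetUnselected switch that widget's selection square between visible and hidden.
; An unconnected color blend from dry to wet ground based on humidity is left unused.
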(event `self.ReceiveBeginPlay`
  (bind _assoil_widget_bp (cast `/Game/Models/Plantes/Soil/Soil_Widget_BP` (`WidgetComponent.GetUserWidgetObject` (`self.Widget`))))
  (set `self.Soil_Widget` _assoil_widget_bp))

(event `self.ReceiveTick`
  (params (DeltaSeconds :type "Float (single-precision)")))

(event `self.SetSelected`
  (set `/Game/Models/Plantes/Soil/Soil_Widget_BP.Selection_Square_Visibility` "Visible" (`self.Soil_Widget`)))

(event `self.SetUnselected`
  (set `/Game/Models/Plantes/Soil/Soil_Widget_BP.Selection_Square_Visibility` "Hidden" (`self.Soil_Widget`)))

(fn `UserConstructionScript`)