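; Corn plant actor that grows through morph target stages and later rots.
; After a hatch delay on BeginPlay it enters the Growing state, which Tick polls every frame.
; Growing runs six chained timelines, driving morph keys 6 down to 1, then waits a rot delay and plays the rot animation.
; The interrupted growth state stops all six timelines.
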(event `self.ReceiveBeginPlay`
  (`KismetSystemLibrary.Delay` (`self.HatchDelay`))
  (set `self.PlantState` "Growing"))

(event `self.ReceiveTick`
  (params (DeltaSeconds :type "Float (single-precision)"))
  (bind _skeletalmeshcomponent (`self.SkeletalMeshComponent`))
  (bind _returnvalue (`self.GetPlantState`))
  (switch `EPlantState` _returnvalue
    (:`Growing`
      (bind (_direction _newtrack_0) (`Timeline|Timeline_0` :!label _label)
        (:`Update`
          (`SkeletalMeshComponent.SetMorphTarget` _skeletalmeshcomponent "Key 6" _newtrack_0 true))
        (:`Finished`
          (bind (_direction_2 _newtrack_0_2) (`Timeline|Timeline_1` :!label _label_2)
            (:`Update`
              (`SkeletalMeshComponent.SetMorphTarget` _skeletalmeshcomponent "Key 5" _newtrack_0_2 true))
            (:`Finished`
              (bind (_direction_3 _newtrack_0_3) (`Timeline|Timeline_2` :!label _label_3)
                (:`Update`
                  (`SkeletalMeshComponent.SetMorphTarget` _skeletalmeshcomponent "Key 4" _newtrack_0_3 true))
                (:`Finished`
                  (bind (_direction_4 _newtrack_0_4) (`Timeline|Timeline_3` :!label _label_4)
                    (:`Update`
                      (`SkeletalMeshComponent.SetMorphTarget` _skeletalmeshcomponent "Key 3" _newtrack_0_4 true))
                    (:`Finished`
                      (bind (_direction_5 _newtrack_0_5) (`Timeline|Timeline_4` :!label _label_5)
                        (:`Update`
                          (`SkeletalMeshComponent.SetMorphTarget` _skeletalmeshcomponent "Key 2" _newtrack_0_5 true))
                        (:`Finished`
                          (bind (_direction_6 _newtrack_0_6) (`Timeline|Timeline_5` :!label _label_6)
                            (:`Update`
                              (`SkeletalMeshComponent.SetMorphTarget` _skeletalmeshcomponent "Key 1" _newtrack_0_6 true))
                            (:`Finished`
                              (`KismetSystemLibrary.Delay` (`self.RotDelay`))
                              (`SkeletalMeshComponent.PlayAnimation` (`self.SkeletalMeshComponent`) "/Game/Models/Plantes/Corn/Corn_Anim_Rot.Corn_Anim_Rot" false))))))))))))))
    (:`InteruptedGrowth`
      (`|ExecutionSequence`
        (:`then_0`
          (goto _label :!via `Stop`))
        (:`then_1`
          (goto _label_2 :!via `Stop`))
        (:`then_2`
          (goto _label_3 :!via `Stop`))
        (:`then_3`
          (goto _label_4 :!via `Stop`))
        (:`then_4`
          (goto _label_5 :!via `Stop`))
        (:`then_5`
          (goto _label_6 :!via `Stop`))))))

(fn `UserConstructionScript`)