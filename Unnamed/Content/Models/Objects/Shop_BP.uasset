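; Shop actor that gives the player access to a shop UI and shifts the character camera near its table.
; On BeginPlay it creates a Shop_Widget_BP and adds it to the viewport.
; OpenShop switches input to UI-only, focused on that widget, and activates it.
; Overlapping the Table component sets a sideways camera offset on Personnage_BP, and leaving restores the default.
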(event `self.ReceiveBeginPlay`
  (bind _returnvalue (`|CreateWidget` "/Game/UI/HUD/Shop/Shop_Widget_BP.Shop_Widget_BP_C"))
  (`UserWidget.AddToViewport` _returnvalue 0))

(event `self.OpenShop`
  (`WidgetBlueprintLibrary.SetInputMode_UIOnlyEx` (`GameplayStatics.GetPlayerController` 0) (stale `self.ReceiveBeginPlay` _returnvalue))
  (`/Game/UI/HUD/Shop/Shop_Widget_BP.Activate` (stale `self.ReceiveBeginPlay` _returnvalue)))

(event `self.Table.OnComponentBeginOverlap`
  (params (OverlappedComponent :type "PrimitiveComponent Object Reference") (OtherActor :type "Actor Object Reference") (OtherComp :type "PrimitiveComponent Object Reference") (OtherBodyIndex :type Integer) (bFromSweep :type Boolean) (SweepResult :type "HitResult Structure (by ref)"))
  (bind _aspersonnage_bp (cast `/Game/Models/Personnage/Personnage_BP` OtherActor))
  (bind (_defaultcameraoffset_x _defaultcameraoffset_y _defaultcameraoffset_z) (`KismetMathLibrary.BreakVector` (`UnnamedCharacter.DefaultCameraOffset` _aspersonnage_bp)))
  (`UnnamedCharacter.SetNewCameraOffset` _aspersonnage_bp (`KismetMathLibrary.MakeVector` _defaultcameraoffset_x -200.0 _defaultcameraoffset_z)))

(event `self.Table.OnComponentEndOverlap`
  (params (OverlappedComponent :type "PrimitiveComponent Object Reference") (OtherActor :type "Actor Object Reference") (OtherComp :type "PrimitiveComponent Object Reference") (OtherBodyIndex :type Integer))
  (bind _aspersonnage_bp (cast `/Game/Models/Personnage/Personnage_BP` OtherActor))
  (`UnnamedCharacter.SetNewCameraOffset` _aspersonnage_bp (`UnnamedCharacter.DefaultCameraOffset` _aspersonnage_bp)))

(fn `UserConstructionScript`)