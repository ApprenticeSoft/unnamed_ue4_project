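; Player character Blueprint with a test event that plays a plant-picking interaction.
; The event locks move input while a timeline turns the actor to a stored yaw angle.
; It then plays pickup animations directly on the mesh, calling PickPlants on the interaction target between the beginning and end clips.
; Fixed delays time each clip before input is restored and the mesh returns to its Animation Blueprint.
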(event `self.Test`
  (bind _returnvalue (`GameplayStatics.GetPlayerController` 0))
  (`Controller.SetIgnoreMoveInput` _returnvalue true)
  ;[1 1 1] Rotation towards target
  (bind (_direction _angle) (`Timeline|Angle_Rotation` :!via `PlayFromStart`)
    (:`Update`
      (`self.K2_SetActorRotation` (`KismetMathLibrary.RLerp` (`self.K2_GetActorRotation`) (`KismetMathLibrary.MakeRotator` 0.0 0.0 (`self.AngleRotation`)) _angle)))
    (:`Finished`
      (`SkeletalMeshComponent.PlayAnimation` (`self.Mesh`) "/Game/Models/Personnage/Personnage_Pick_up_beginning.Personnage_Pick_up_beginning" false)
      (`KismetSystemLibrary.Delay` 0.792)
      (`self.PickPlants` (`self.InteractionTarget`))
      (`SkeletalMeshComponent.PlayAnimation` (`self.Mesh`) "/Game/Models/Personnage/Personnage_Pick_up_end.Personnage_Pick_up_end" false)
      (`KismetSystemLibrary.Delay` 0.75)
      (`Controller.ResetIgnoreMoveInput` _returnvalue)
      (`SkeletalMeshComponent.SetAnimationMode` (`self.Mesh`) "AnimationBlueprint"))))

(fn `UserConstructionScript`)