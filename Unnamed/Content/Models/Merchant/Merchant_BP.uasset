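; Merchant character Blueprint whose UpdateSlate event makes the merchant walk to an interaction target and pick a slate.
; One timeline drives MoveToLocation each update until it returns false, then stops and starts a second timeline that lerps the yaw to AngleRotation.
; That timeline's update also plays the pick animation directly on the mesh, then a delay restores Animation Blueprint mode and clears IsBusy.
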(event `self.UpdateSlate`
  (set `self.IsBusy` true)
  (`Timeline|Timeline_1` :!via `PlayFromStart` :!label _label
    (:`Update`
      (bind _returnvalue (`self.MoveToLocation` (`self.InteractionTarget`) 70.0))
      (if (not _returnvalue)
        (`|ExecutionSequence`
          (:`then_0`
            (goto _label :!via `Stop`))
          (:`then_1`
            (bind (_direction _angle) (`Timeline|Timeline_0` :!via `PlayFromStart`)
              (:`Update`
                (`self.K2_SetActorRotation` (`KismetMathLibrary.RLerp` (`self.K2_GetActorRotation`) (`KismetMathLibrary.MakeRotator` 0.0 0.0 (`self.AngleRotation`)) _angle))
                (`SkeletalMeshComponent.PlayAnimation` (`self.Mesh`) "/Game/Models/Merchant/Merchant_Anim_Pick_Slate.Merchant_Anim_Pick_Slate" false)
                (`KismetSystemLibrary.Delay` 2.083)
                (`SkeletalMeshComponent.SetAnimationMode` (`self.Mesh`) "AnimationBlueprint")
                (set `self.IsBusy` false)))))))))

(fn `UserConstructionScript`)